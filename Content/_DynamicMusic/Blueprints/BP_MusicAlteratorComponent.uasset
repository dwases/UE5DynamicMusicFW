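; BP_MusicAlteratorComponent is a component that exposes control of a dynamic, multi-track music system through a music manager passed into each call.
; InitiateSong terminates the current music, stores the new track set and hands it to the manager.
; TerminateMusic deactivates and resets every valid playing sound, then clears the manager's sound and track lists.
; The remaining functions forward track playback, switching, deactivation and maximum-timestamp requests directly to the manager.
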(fn `DeactivateAllTracks`
  (params (`Target Music Manager` :type "/Game/_DynamicMusic/Blueprints/BP_MusicManagerComponent Object Reference"))
  (`/Game/_DynamicMusic/Blueprints/BP_MusicManagerComponent.DeactivateAllTracks` `Target Music Manager`))

(fn `InitiateSong`
  (params (Tracks :type "Array of SoundBase Object Reference") (TargetMusicManager :type "/Game/_DynamicMusic/Blueprints/BP_MusicManagerComponent Object Reference"))
  (`self.TerminateMusic` TargetMusicManager)
  (bind _output_get (set `self.Tracks` Tracks))
  (`/Game/_DynamicMusic/Blueprints/BP_MusicManagerComponent.SetCurrentTracks` TargetMusicManager _output_get))

(fn `PlayAllTracksFromStart`
  (params (TargetMusicManager :type "/Game/_DynamicMusic/Blueprints/BP_MusicManagerComponent Object Reference"))
  (`/Game/_DynamicMusic/Blueprints/BP_MusicManagerComponent.PlayAllTracksFromStart` TargetMusicManager))

(fn `PlayAllTracksFromTimestamp`
  (params (TargetMusicManager :type "/Game/_DynamicMusic/Blueprints/BP_MusicManagerComponent Object Reference") (Timestamp :type "Float (double-precision)"))
  (`/Game/_DynamicMusic/Blueprints/BP_MusicManagerComponent.Play All Tracks from Timestamp` TargetMusicManager Timestamp))

(fn `PlaySelectTracksFromStart`
  (params (TargetMusicManager :type "/Game/_DynamicMusic/Blueprints/BP_MusicManagerComponent Object Reference") (TrackNumbers :type "Array of Integer"))
  (`/Game/_DynamicMusic/Blueprints/BP_MusicManagerComponent.PlaySelectTracksFromStart` TargetMusicManager TrackNumbers))

(fn `PlaySelectTracksFromTimestamp`
  (params (TargetMusicManager :type "/Game/_DynamicMusic/Blueprints/BP_MusicManagerComponent Object Reference") (TrackNumbers :type "Array of Integer") (Timestamp :type "Float (double-precision)"))
  (`/Game/_DynamicMusic/Blueprints/BP_MusicManagerComponent.PlaySelectTracksFromTimestamp` TargetMusicManager TrackNumbers Timestamp))

(fn `SetMaxTimestamp`
  (params (TargetMusicManager :type "/Game/_DynamicMusic/Blueprints/BP_MusicManagerComponent Object Reference") (MaxTimestamp :type "Float (double-precision)"))
  (`/Game/_DynamicMusic/Blueprints/BP_MusicManagerComponent.SetMaxTimestamp` TargetMusicManager MaxTimestamp))

(fn `SwitchToSelectTracks`
  (params (`Target Music Manager` :type "/Game/_DynamicMusic/Blueprints/BP_MusicManagerComponent Object Reference") (TrackNumbers :type "Array of Integer"))
  (`/Game/_DynamicMusic/Blueprints/BP_MusicManagerComponent.SwitchToSelectTracks` `Target Music Manager` TrackNumbers))

(fn `TerminateMusic`
  (params (TargetMusicManager :type "/Game/_DynamicMusic/Blueprints/BP_MusicManagerComponent Object Reference"))
  (for _array_element (`/Game/_DynamicMusic/Blueprints/BP_MusicManagerComponent.PlayingSounds` TargetMusicManager)
    (`/Engine/EditorBlueprintResources/StandardMacros.IsValid` _array_element
      (:`Is Valid`
        (`self.SetActive` _array_element false true))))
  (set `/Game/_DynamicMusic/Blueprints/BP_MusicManagerComponent.PlayingSounds` (`|MakeArray`) TargetMusicManager)
  (`/Game/_DynamicMusic/Blueprints/BP_MusicManagerComponent.SetCurrentTracks` TargetMusicManager (`|MakeArray`)))